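; Trigger volume that shows a tutorial and unlocks the matching player ability when BP_Player overlaps its box.
; It passes its Tutorial value to the custom player controller, deactivates any active widget in the Totu container and adds WBP_Tutorial there.
; A switch on Tutorial calls DoubleJump on the player's skills or sets the Finisher or Homing unlock flag.
; Nothing disables the trigger, so each new overlap repeats the sequence.
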(event OnComponentBeginOverlap(Box)
  (params (OverlappedComponent :type Primitive%20Component%20Object%20Reference) (OtherActor :type Actor%20Object%20Reference) (OtherComp :type Primitive%20Component%20Object%20Reference) (OtherBodyIndex :type Integer) (bFromSweep :type Boolean) (SweepResult :type Hit%20Result%20Structure%20%28by%20ref%29))
  (bind _asbp_player (Utilities|Casting|CastToBP_Player OtherActor))
  (Variables|Default|Setplayer _asbp_player)
  (bind _asbp_custom_player_controller (Utilities|Casting|CastToBP_CustomPlayerController (Game|GetPlayerController 0)))
  (Variables|/Game/Blueprints/BP_CustomPlayerController.BP_CustomPlayerController_C|SetTutorial _asbp_custom_player_controller (Variables|Default|GetTutorial))
  (Utilities|IsValid (Class|CommonActivatableWidgetContainerBase|GetActiveWidget (Variables|/Game/Blueprints/Widgets/WBP_CommonBase.WBP_CommonBase_C|GetTotu (Variables|/Game/Blueprints/BP_CustomPlayerController.BP_CustomPlayerController_C|GetWidgetBaseRef _asbp_custom_player_controller)))
    (:Is%20Valid
      (Class|CommonActivatableWidget|DeactivateWidget (Class|CommonActivatableWidgetContainerBase|GetActiveWidget (Variables|/Game/Blueprints/Widgets/WBP_CommonBase.WBP_CommonBase_C|GetTotu (Variables|/Game/Blueprints/BP_CustomPlayerController.BP_CustomPlayerController_C|GetWidgetBaseRef _asbp_custom_player_controller)))))
    (:Is%20Not%20Valid
      _))
  (Class|CommonActivatableWidgetContainerBase|AddWidget (Variables|/Game/Blueprints/Widgets/WBP_CommonBase.WBP_CommonBase_C|GetTotu (Variables|/Game/Blueprints/BP_CustomPlayerController.BP_CustomPlayerController_C|GetWidgetBaseRef _asbp_custom_player_controller)) "/Game/Blueprints/Widgets/WBP_Tutorial.WBP_Tutorial_C")
  (switch Utilities|FlowControl|Switch|SwitchonETutorials (Variables|Default|GetTutorial)
    (:NewEnumerator5
      (Default|DoubleJump (Variables|/Game/Blueprints/Player/BP_Player.BP_Player_C|GetSkillsRef (Variables|Default|Getplayer))))
    (:NewEnumerator7
      (Variables|/Game/Blueprints/Player/BP_Player.BP_Player_C|SetFinisherUnlocked (Variables|Default|Getplayer) true))
    (:NewEnumerator8
      (Variables|/Game/Blueprints/Player/BP_Player.BP_Player_C|SetHomingUnlocked (Variables|Default|Getplayer) true))))

(fn ConstructionScript)