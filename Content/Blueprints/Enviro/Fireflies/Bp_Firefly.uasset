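; Firefly actor that drives a Niagara effect, fading it in and out in an endless loop within a spawner's box.
; After a random startup delay, a timeline at a random play rate lerps the Niagara AlphaScale parameter.
; A FlipFlop on timeline completion alternates between reversing to fade out and, while invisible, teleporting to a random point inside the Spawner's box bounds before fading in again.
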(event EventBeginPlay
  (bind _fadetimeline (Variables|Default|GetFAdeTimeline))
  (bind _spawner (Variables|Default|GetSpawner))
  (Utilities|FlowControl|Delay (Math|Random|RandomFloatinRange 0.0 1e+01))
  (Components|Timeline|SetPlayRate (Variables|Default|GetFAdeTimeline) (Math|Random|RandomFloatinRange 0.1 0.5))
  (bind _newtrack_0 (Timeline|FAdeTimeline PlayFromStart)
    (:Update
      (Effects|Components|ParticleSystem|SetFloatParameter (Variables|Default|GetNiagara) "AlphaScale" (Math|Float|Lerp 0.0 1.0 _newtrack_0)))
    (:Finished
      (Utilities|FlowControl|FlipFlop
        (:A
          (Components|Timeline|ReversefromEnd _fadetimeline))
        (:B
          (Transformation|SetActorLocation (Math|Random|RandomPointinBoundingBox (Transformation|GetActorLocation _spawner) (Variables|/Script/Engine.BoxComponent|GetBoxExtent (Variables|/Game/Blueprints/Enviro/Fireflies/BP_FireflyArea.BP_FireflyArea_C|GetBox _spawner))) false false)
          (Components|Timeline|PlayfromStart _fadetimeline))))))

(event Collision|EventActorBeginOverlap
  (params (OtherActor :type Actor%20Object%20Reference)))

(event EventTick
  (params (DeltaSeconds :type Float%20%28single-precision%29)))

(fn ConstructionScript)