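; BP_FireflyArea is an environment effect that surrounds the player with fireflies.
; On BeginPlay it attaches itself to player 0's character and sets a relative offset above it, so the area travels with the player.
; It then spawns Quantity Bp_Firefly actors at random points within its Box extent, passing itself to each as Spawner.
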(event Custom|Spawn
  (Game|SpawnActorfromClass "/Game/Blueprints/Enviro/Fireflies/Bp_Firefly.Bp_Firefly_C" (Math|Transform|MakeTransform (Math|Random|RandomPointinBoundingBox (Transformation|GetActorLocation) (Variables|/Script/Engine.BoxComponent|GetBoxExtent (Variables|Default|GetBox))) "0, 0, 0" "1.000000,1.000000,1.000000") "Undefined" 0 self 0))

(event EventBeginPlay
  (Transformation|AttachActorToActor (Game|GetPlayerCharacter 0) "None" "SnapToTarget" "SnapToTarget" "KeepWorld" false)
  (Transformation|SetActorRelativeLocation "0, 0,300.000000")
  (for _index (range 1 (Variables|Default|Getquantity))
    (CallFunction|Spawn)))

(fn ConstructionScript)