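; Environment spline actor, named as a root (racine), that lays copies of a mesh along its spline as collidable spline mesh segments hidden in game.
; The construction script loops by spline point count, but places segments by distance, advancing by the mesh's X-axis bounds length each step.
; Info supplies local location and tangent at each segment's ends, and Size derives that length from the mesh bounding box.
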(event EventBeginPlay)

(event Collision|EventActorBeginOverlap
  (params (OtherActor :type Actor%20Object%20Reference)))

(event EventTick
  (params (DeltaSeconds :type Float%20%28single-precision%29)))

(fn ConstructionScript
  (for _index (range 0 (Spline|GetNumberOfSplinePoints (Variables|Default|GetSpline)))
    (LocalVariables|SetStartLoc (.LocDist (CallFunction|Info (LocalVariables|GetActualDist) _index)))
    (LocalVariables|SetStartTang (.TangDist (CallFunction|Info (LocalVariables|GetActualDist) _index)))
    (LocalVariables|SetActualDist (+ (CallFunction|Size) (LocalVariables|GetActualDist)))
    (LocalVariables|SetEndLoc (.LocDist (CallFunction|Info (LocalVariables|GetActualDist) _index)))
    (LocalVariables|SetEndTang (.TangDist (CallFunction|Info (LocalVariables|GetActualDist) _index)))
    (bind _returnvalue (AddComponent|AddSplineMeshComponent false (Math|Transform|MakeTransform "0, 0, 0" "0.000000,90.000000,0.000000" "1.000000,1.000000,1.000000")))
    (LocalVariables|SetCurrentSplineMesh _returnvalue)
    (Components|StaticMesh|SetStaticMesh (LocalVariables|GetCurrentSplineMesh) (Variables|Default|GetMesh))
    (Collision|SetCollisionEnabled (LocalVariables|GetCurrentSplineMesh) "QueryAndPhysics")
    (SplineMesh|SetForwardAxis (LocalVariables|GetCurrentSplineMesh) "X" true)
    (SplineMesh|SetStartandEnd (LocalVariables|GetCurrentSplineMesh) (LocalVariables|GetStartLoc) (LocalVariables|GetStartTang) (LocalVariables|GetEndLoc) (LocalVariables|GetEndTang) true :!class /Script/Engine.SplineMeshComponent)
    (Development|SetHiddeninGame (LocalVariables|GetCurrentSplineMesh) true false)))

(fn Info
  (params (Distance :type Float%20%28single-precision%29) (PointInd :type Integer))
  (bind _spline (Variables|Default|GetSpline))
  (return (Spline|GetLocationatDistanceAlongSpline _spline Distance "Local") (Spline|GetTangentatDistanceAlongSpline _spline Distance "Local") (Spline|GetLocationatSplinePoint _spline PointInd "Local") (Spline|GetTangentatSplinePoint _spline PointInd "Local")))

(fn Size
  (bind _mesh (Variables|Default|GetMesh))
  (bind _returnvalue (StaticMesh|GetBoundingBox _mesh))
  (return (+ (Math|Float|Absolute(Float) (Utilities|Select :Index "X" :X (.x (.min _returnvalue)) :Y (.y (.min _returnvalue)) :Z (.z (.min _returnvalue)))) (Math|Float|Absolute(Float) (Utilities|Select :Index "X" :X (.x (.max _returnvalue)) :Y (.y (.max _returnvalue)) :Z (.z (.max _returnvalue)))))))