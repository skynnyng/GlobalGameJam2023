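; Grapple actor that attaches to the player's left hand with a cable and lets the player grab grapple points.
; On BeginPlay it gathers all grapple points in the level, snaps to the hand socket and registers itself on the player.
; StartGrab plays a sound and triggers the reachable point closest to screen center, unless already grappling.
; A short timer event restores the player's gravity scale.
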(event Custom|StartGrab
  (if (and (Utilities|Array|IsNotEmpty (Variables|Default|GetGrapplePointsReachable)) (not (Variables|Default|GetinGrapple)))
    (Variables|Default|SetinGrapple true)
    (Audio|Components|Audio|Play (Variables|Default|GetSound) 0.0)
    (bind _asbp_grapple_point (Utilities|Casting|CastToBP_GrapplePoint (CallFunction|FincClosestActortoCenterOfScreen (Variables|Default|GetGrapplePointsReachable) self)))
    (Default|StartGrab _asbp_grapple_point)))

(event Custom|ResetGravityTimerEvent
  (bind _returnvalue (Utilities|Time|SetTimerbyEvent (delegate Custom|ResetGravity) 0.2))
  (Variables|Default|SetResetGravityTimer _returnvalue))

(event Custom|ResetGravity
  (Variables|/Script/Engine.CharacterMovementComponent|SetGravityScale (Variables|/Script/Engine.Character|GetCharacterMovement (Variables|Default|GetplayerRef)) 1e+01))

(event EventBeginPlay
  (bind _outactors (Actor|GetAllActorsOfClass "/Game/Blueprints/Interactible/BP_GrapplePoint.BP_GrapplePoint_C"))
  (Variables|Default|SetGrapplePoints _outactors)
  (bind _asbp_player (Utilities|Casting|CastToBP_Player (Game|GetPlayerCharacter 0)))
  (Variables|Default|SetplayerRef _asbp_player)
  (Transformation|AttachComponentToComponent (Variables|/Script/Engine.Character|GetMesh (Variables|Default|GetplayerRef)) "LeftHandSocket" "SnapToTarget" "SnapToTarget" "KeepRelative" true)
  (Class|CableComponent|SetAttachEndtoComponent (Variables|Default|GetCableComponent) (Variables|/Script/Engine.Character|GetMesh (Variables|Default|GetplayerRef)) "LeftHandSocket")
  (Variables|/Game/Blueprints/Player/BP_Player.BP_Player_C|SetGrapple (Variables|Default|GetplayerRef) self))

(fn ConstructionScript)