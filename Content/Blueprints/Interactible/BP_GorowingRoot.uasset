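; Interactible root actor, apparently meant to grow and wither, built from spline meshes laid along a spline.
; The construction script splits the spline into sections scaled by actor X scale, storing each mesh with its endpoints and length-clamped tangents in the Splin array.
; Each section follows the spline's position and roll and is set visible.
; BeginPlay, Grow and Wither are empty stubs, so no runtime animation exists here.
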(event Custom|Grow
  ;[1 1 1] Grow
)

(event Custom|Wither
  ;[1 1 1] Wither
)

(event EventBeginPlay
  ;[1 1 1] PlayRate
)

(fn ConstructionScript
  (Variables|Default|SetsectionLength (* (.x (Transformation|GetActorScale3D)) (Variables|Default|GetsectionLength)))
  (for _index (range 0 (Math|Float|Truncate (/ (Spline|GetSplineLength (Variables|Default|GetSpline)) (Variables|Default|GetsectionLength))))
    (Variables|Default|SetpointIndex _index)
    (bind _returnvalue (AddComponent|AddSplineMeshComponent false))
    (Utilities|Array|Add (Variables|Default|Getsplin) (Utilities|Struct|MakeSplineMeshInfos _returnvalue (Spline|GetLocationatDistanceAlongSpline (Variables|Default|GetSpline) (* (Variables|Default|GetpointIndex) (Variables|Default|GetsectionLength)) "Local") (Math|Vector|ClampVectorSize (Spline|GetTangentatDistanceAlongSpline (Variables|Default|GetSpline) (* (Variables|Default|GetpointIndex) (Variables|Default|GetsectionLength)) "Local") 0.0 (Variables|Default|GetsectionLength)) (Spline|GetLocationatDistanceAlongSpline (Variables|Default|GetSpline) (* (+ (Variables|Default|GetpointIndex) 1) (Variables|Default|GetsectionLength)) "Local") (Math|Vector|ClampVectorSize (Spline|GetTangentatDistanceAlongSpline (Variables|Default|GetSpline) (* (+ (Variables|Default|GetpointIndex) 1) (Variables|Default|GetsectionLength)) "Local") 0.0 (Variables|Default|GetsectionLength))))
    (SplineMesh|SetStartandEnd (.splinemesh (Utilities|Array|Get(acopy) (Variables|Default|Getsplin) (Variables|Default|GetpointIndex))) (.startpos (Utilities|Array|Get(acopy) (Variables|Default|Getsplin) (Variables|Default|GetpointIndex))) (.starttan (Utilities|Array|Get(acopy) (Variables|Default|Getsplin) (Variables|Default|GetpointIndex))) (.endpos (Utilities|Array|Get(acopy) (Variables|Default|Getsplin) (Variables|Default|GetpointIndex))) (.endtan (Utilities|Array|Get(acopy) (Variables|Default|Getsplin) (Variables|Default|GetpointIndex))) true :!class /Script/Engine.SplineMeshComponent)
    (Class|SplineMeshComponent|SetStartRoll (.splinemesh (Utilities|Array|Get(acopy) (Variables|Default|Getsplin) (Variables|Default|GetpointIndex))) (Math|Trig|DegreesToRadians (Class|SplineComponent|GetRollatDistanceAlongSpline (Variables|Default|GetSpline) (* (Variables|Default|GetpointIndex) (Variables|Default|GetsectionLength)) "Local")) true)
    (Class|SplineMeshComponent|SetEndRoll (.splinemesh (Utilities|Array|Get(acopy) (Variables|Default|Getsplin) (Variables|Default|GetpointIndex))) (Math|Trig|DegreesToRadians (Class|SplineComponent|GetRollatDistanceAlongSpline (Variables|Default|GetSpline) (* (+ (Variables|Default|GetpointIndex) 1) (Variables|Default|GetsectionLength)) "Local")) true)
    (Rendering|SetVisibility (.splinemesh (Utilities|Array|Get(acopy) (Variables|Default|Getsplin) (Variables|Default|GetpointIndex))) true false)))