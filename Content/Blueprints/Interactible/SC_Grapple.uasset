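; SC_Grapple is a scene component that starts a grab on the nearest reachable grapple point.
; On BeginPlay it caches every BP_GrapplePoint actor in the level into GrapplePoints.
; StartGrab finds the actor in GrapplePointsReachable closest to the component's world location and calls that point's own StartGrab, leaving the grab itself to the point.
; This graph only reads GrapplePointsReachable and never fills it.
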(event Custom|StartGrab
  (if (Utilities|Array|IsNotEmpty (Variables|Default|GetGrapplePointsReachable))
    (bind _asbp_grapple_point (Utilities|Casting|CastToBP_GrapplePoint (.ReturnValue (Actor|FindNearestActor (Transformation|GetWorldLocation) (Variables|Default|GetGrapplePointsReachable)))))
    (Default|StartGrab _asbp_grapple_point)))

(event EventBeginPlay
  (bind _outactors (Actor|GetAllActorsOfClass "/Game/Blueprints/Interactible/BP_GrapplePoint.BP_GrapplePoint_C"))
  (Variables|Default|SetGrapplePoints _outactors))