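; C_Interactible is a component for focusable, targetable interactibles, but its events are empty and nearly all its logic sits disconnected.
; The unwired code adds an owner-sized overlap box, switches its trace channel for targetability, and shows a bobbing, camera-facing arrow.
; Other stranded fragments forward damage to the owner and display debug text, with several cast classes missing.
; Only CheckBrothers is intact, reporting whether any sibling component can be focused.
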(event Custom|isFocused)

(event Custom|Unfocused)

(event Custom|MakeNotTargetable)

(event Custom|MakeTargetable)

(event Custom|PlayerBeginPlay)

(event Custom|DamageOwner
  (params (Damage :type Float%20%28double-precision%29) (Controller :type Controller%20Object%20Reference) (Instigator :type Actor%20Object%20Reference) (DamageType :type Damage%20Type%20Class%20Reference) (Normal :type Vector) (ImpactLocation :type Vector)))

(event EventBeginPlay)

(event EventTick
  (params (DeltaSeconds :type Float%20%28single-precision%29)))

(fn Debug)

(fn CheckBrothers
  (for _array_element (Actor|GetComponentsByClass (Components|GetOwner) "C_Interactible_C")
    (if (Variables|C_Interactible_C|GetcanFocus _array_element)
      (return true)))
  (return false))