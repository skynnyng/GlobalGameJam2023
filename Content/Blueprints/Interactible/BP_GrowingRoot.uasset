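; BP_GrowingRoot is an interactible root built from spline mesh segments along a spline, shown or hidden by its Grown flag.
; The construction script scales SectionLength by actor X scale, then adds a movable mesh per section, storing each with positions and tangents in the Splin array.
; Roll follows the spline.
; Both tangents sample the section's start, with only the start tangent clamped to section length.
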(fn ConstructionScript
  (Variables|Default|SetsectionLength (* (.x (Transformation|GetActorScale3D)) (Variables|Default|GetsectionLength)))
  (for _index (range 0 (Math|Float|Truncate (/ (Spline|GetSplineLength (Variables|Default|GetSpline)) (Variables|Default|GetsectionLength))))
    (Variables|Default|SetpointIndex _index)
    (bind _returnvalue (AddComponent|AddSplineMeshComponent false))
    (Utilities|Array|Add (Variables|Default|Getsplin) (Utilities|Struct|MakeSplineMeshInfos _returnvalue (Spline|GetLocationatDistanceAlongSpline (Variables|Default|GetSpline) (* (Variables|Default|GetpointIndex) (Variables|Default|GetsectionLength)) "Local") (Math|Vector|ClampVectorSize (Spline|GetTangentatDistanceAlongSpline (Variables|Default|GetSpline) (* (Variables|Default|GetpointIndex) (Variables|Default|GetsectionLength)) "Local") 0.0 (Variables|Default|GetsectionLength)) (Spline|GetTangentatDistanceAlongSpline (Variables|Default|GetSpline) (* (Variables|Default|GetpointIndex) (Variables|Default|GetsectionLength)) "Local") (Spline|GetLocationatDistanceAlongSpline (Variables|Default|GetSpline) (* (+ (Variables|Default|GetpointIndex) 1) (Variables|Default|GetsectionLength)) "Local")))
    (Transformation|SetMobility (.splinemesh (Utilities|Array|Get(acopy) (Variables|Default|Getsplin) (Variables|Default|GetpointIndex))) "Movable")
    (SplineMesh|SetStartandEnd (.splinemesh (Utilities|Array|Get(acopy) (Variables|Default|Getsplin) (Variables|Default|GetpointIndex))) (.startpos (Utilities|Array|Get(acopy) (Variables|Default|Getsplin) (Variables|Default|GetpointIndex))) (.starttan (Utilities|Array|Get(acopy) (Variables|Default|Getsplin) (Variables|Default|GetpointIndex))) (.endpos (Utilities|Array|Get(acopy) (Variables|Default|Getsplin) (Variables|Default|GetpointIndex))) (.endtan (Utilities|Array|Get(acopy) (Variables|Default|Getsplin) (Variables|Default|GetpointIndex))) true :!class /Script/Engine.SplineMeshComponent)
    (Components|StaticMesh|SetStaticMesh (.splinemesh (Utilities|Array|Get(acopy) (Variables|Default|Getsplin) (Variables|Default|GetpointIndex))) (Variables|Default|GetmeshSection))
    (SplineMesh|SetForwardAxis (.splinemesh (Utilities|Array|Get(acopy) (Variables|Default|Getsplin) (Variables|Default|GetpointIndex))) (Variables|Default|GetmeshForwardAxis) true)
    (Class|SplineMeshComponent|SetStartRoll (.splinemesh (Utilities|Array|Get(acopy) (Variables|Default|Getsplin) (Variables|Default|GetpointIndex))) (Math|Trig|DegreesToRadians (Class|SplineComponent|GetRollatDistanceAlongSpline (Variables|Default|GetSpline) (* (Variables|Default|GetpointIndex) (Variables|Default|GetsectionLength)) "Local")) true)
    (Class|SplineMeshComponent|SetEndRoll (.splinemesh (Utilities|Array|Get(acopy) (Variables|Default|Getsplin) (Variables|Default|GetpointIndex))) (Math|Trig|DegreesToRadians (Class|SplineComponent|GetRollatDistanceAlongSpline (Variables|Default|GetSpline) (* (+ (Variables|Default|GetpointIndex) 1) (Variables|Default|GetsectionLength)) "Local")) true)
    (Rendering|SetVisibility (.splinemesh (Utilities|Array|Get(acopy) (Variables|Default|Getsplin) (Variables|Default|GetpointIndex))) true false))
  (for _array_element (Variables|Default|Getsplin)
    (Rendering|SetVisibility (.splinemesh _array_element) (Variables|Default|GetGrown) false)))