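; Grapple point actor that pulls the player toward itself with their grapple.
; Tick adds or removes it from the Grapple's reachable list by player distance and on-screen visibility.
; StartGrab halts walking and gravity, then a timeline flies the detached hook to the point while turning the player, finally moving and launching them before reattaching the hook.
; A dynamic material lets ChangeEmissive toggle glow; montage-driven start logic is left unconnected.
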(event Custom|StartGrab
  (bind _returnvalue (Transformation|GetActorLocation))
  (bind _player (Variables|Default|Getplayer))
  (bind _player_2 (Variables|Default|Getplayer))
  (bind _returnvalue_2 (Transformation|GetActorLocation _player_2))
  (Variables|/Script/Engine.CharacterMovementComponent|SetMaxWalkSpeed (Variables|/Script/Engine.Character|GetCharacterMovement (Variables|Default|Getplayer)) 0.0)
  (Utilities|FlowControl|Delay 0.25)
  (Variables|/Script/Engine.CharacterMovementComponent|SetGravityScale (Variables|/Script/Engine.Character|GetCharacterMovement (Variables|Default|Getplayer)) 0.0)
  (Transformation|DetachFromComponent (Variables|/Script/Engine.Actor|GetRootComponent (Variables|Default|Getgrapple)) "KeepWorld" "KeepWorld" "KeepWorld" true)
  (Rendering|SetVisibility (Variables|/Script/Engine.Actor|GetRootComponent (Variables|Default|Getgrapple)) true true)
  (Variables|Default|SetLocationSelf (Transformation|GetActorLocation))
  (Variables|Default|SetLocationGrapple (Transformation|GetWorldLocation (Variables|/Script/Engine.Actor|GetRootComponent (Variables|Default|Getgrapple))))
  (Variables|/Script/Engine.MovementComponent|SetVelocity (Variables|/Script/Engine.Character|GetCharacterMovement _player) (* (Math|Vector|GetUnitDirection(Vector) (Transformation|GetActorLocation _player) (Transformation|GetWorldLocation (Variables|Default|GetC_Interactible))) 1e+01))
  (bind _newtrack_0 (Timeline|GrappleTimeline PlayFromStart)
    (:Update
      (Transformation|SetWorldLocation (Variables|/Script/Engine.Actor|GetRootComponent (Variables|Default|Getgrapple)) (Math|Vector|Lerp(Vector) (Variables|Default|GetLocationGrapple) (Variables|Default|GetLocationSelf) _newtrack_0) false false)
      (Transformation|SetActorRotation (Variables|Default|Getplayer) (Math|Rotator|MakeRotator 0.0 0.0 (.yaw (Math|Rotator|Lerp(Rotator) (Pawn|GetControlRotation (Game|GetPlayerController 0) :!class /Script/Engine.Controller) (Math|Rotator|FindLookatRotation (Transformation|GetActorLocation (Variables|Default|Getplayer)) (Transformation|GetActorLocation)) _newtrack_0 true)))))
    (:Finished
      (Variables|Default|Setdistance (Math|Vector|Distance(Vector) _returnvalue_2 _returnvalue))
      (Variables|Default|Setdirection (Math|Vector|GetForwardVector (Math|Rotator|FindLookatRotation _returnvalue_2 _returnvalue)))
      (Components|MoveComponentTo (Variables|/Script/Engine.Character|GetCapsuleComponent (Variables|Default|Getplayer)) (Math|Vector|Lerp(Vector) (Transformation|GetActorLocation (Variables|Default|Getplayer)) (Transformation|GetActorLocation) 0.8) "0, 0, 0" true false 0.2 false)
      (Character|LaunchCharacter (Variables|Default|Getplayer) (Math|Vector|MakeVector (.x (* (Variables|Default|Getdirection) (/ (Variables|Default|Getdistance) 3.0))) (.y (* (Variables|Default|Getdirection) (/ (Variables|Default|Getdistance) 3.0))) (.z (* (Variables|Default|Getdirection) (/ (Variables|Default|Getdistance) 1.5)))) true true)
      (Variables|/Script/Engine.CharacterMovementComponent|SetMaxWalkSpeed (Variables|/Script/Engine.Character|GetCharacterMovement (Variables|Default|Getplayer)) 2.4e+03)
      (Rendering|SetVisibility (Variables|/Script/Engine.Actor|GetRootComponent (Variables|Default|Getgrapple)) false true)
      (Transformation|SetWorldLocation (Variables|/Script/Engine.Actor|GetRootComponent (Variables|Default|Getgrapple)) (Transformation|GetActorLocation (Variables|Default|Getplayer)) false false)
      (Transformation|AttachComponentToComponent (Variables|/Script/Engine.Actor|GetRootComponent (Variables|Default|Getgrapple)) (Variables|/Script/Engine.Character|GetMesh (Variables|Default|Getplayer)) "LeftHandSocket" "SnapToTarget" "SnapToTarget" "KeepWorld" true)
      (Default|ResetGravityTimerEvent (Variables|Default|Getgrapple))
      (Variables|/Game/Blueprints/Interactible/CA_Grapple.CA_Grapple_C|SetinGrapple (Variables|Default|Getgrapple) false))))

(event EventBeginPlay
  (bind _asbp_player (Utilities|Casting|CastToBP_Player (Game|GetPlayerCharacter 0)))
  (Variables|Default|Setplayer _asbp_player)
  (Variables|Default|SetplayerController (Game|GetPlayerController 0))
  (Variables|Default|Setgrapple (Variables|/Game/Blueprints/Player/BP_Player.BP_Player_C|GetGrapple (Variables|Default|Getplayer)))
  (Variables|Default|SetLocationSelf (Transformation|GetActorLocation))
  (Actor|Tick|SetActorTickEnabled true))

(event EventTick
  (params (DeltaSeconds :type Float%20%28single-precision%29))
  (bind _self self)
  (bind _self_2 self)
  (bind _player (Variables|Default|Getplayer))
  (bind _returnvalue (Transformation|GetDistanceTo _player _self_2))
  (Variables|Default|Setgrapple (Variables|/Game/Blueprints/Player/BP_Player.BP_Player_C|GetGrapple (Variables|Default|Getplayer)))
  (if (and (and (> _returnvalue 5e+02) (< _returnvalue 3.5e+03)) (CallFunction|IsLocationonScreen (Variables|Default|GetLocationSelf)))
    (Utilities|Array|AddUnique (Variables|/Game/Blueprints/Interactible/CA_Grapple.CA_Grapple_C|GetGrapplePointsReachable (Variables|Default|Getgrapple)) _self)
    (else
      (bind _grapple (Variables|Default|Getgrapple)
        (:then
          (if (Utilities|Array|ContainsItem (Variables|/Game/Blueprints/Interactible/CA_Grapple.CA_Grapple_C|GetGrapplePointsReachable _grapple) self)
            (Utilities|Array|RemoveItem (Variables|/Game/Blueprints/Interactible/CA_Grapple.CA_Grapple_C|GetGrapplePointsReachable (Variables|Default|Getgrapple)) _self)))
        (:else)))))

(fn ConstructionScript
  (bind _returnvalue (Rendering|Material|CreateDynamicMaterialInstance (Variables|Default|GetSphere) 0 "/Game/Assets/Meshes/Drakkar/INST_Drakkar.INST_Drakkar" "None" :!class /Script/Engine.PrimitiveComponent))
  (Variables|Default|SetInstMat _returnvalue))

(fn ChangeEmissive
  (Utilities|FlowControl|FlipFlop
    (:A
      (Rendering|Material|SetScalarParameterValue (Variables|Default|GetInstMat) "Emissive" 2e+02 :!class /Script/Engine.MaterialInstanceDynamic))
    (:B
      (Rendering|Material|SetScalarParameterValue (Variables|Default|GetInstMat) "Emissive" 0.01 :!class /Script/Engine.MaterialInstanceDynamic))))