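; Snake pursuer that spawns at the end of RacineRef's spline and, after StartGame, homes straight onto the player.
; A timer ramps its per-tick step up to a cap changed after a delay, plus a rubber-band bonus that grows while the player is far and decays when close.
; Touching the player freezes input, switches to the snake's detached camera, plays a lunge, fades to black and opens MainMap.
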(event OnComponentBeginOverlap(Box)
  (params (OverlappedComponent :type Primitive%20Component%20Object%20Reference) (OtherActor :type Actor%20Object%20Reference) (OtherComp :type Primitive%20Component%20Object%20Reference) (OtherBodyIndex :type Integer) (bFromSweep :type Boolean) (SweepResult :type Hit%20Result%20Structure%20%28by%20ref%29))
  (bind _returnvalue (Game|GetPlayerController 0))
  (Utilities|Casting|CastToBP_Player OtherActor)
  (Transformation|DetachFromComponent (Variables|Default|GetCamera) "KeepWorld" "KeepWorld" "KeepWorld" true)
  (Game|Player|SetViewTargetwithBlend _returnvalue self 0.0 "VTBlend_Linear" 0.0 false)
  (Input|DisableInput (Game|GetPlayerCharacter 0) _returnvalue)
  (Actor|Tick|SetActorTickEnabled false)
  (Utilities|FlowControl|Sequence
    (:then_0
      (Timeline|MiamTimeline PlayFromStart
        (:Update
          (Transformation|AddActorWorldOffset (* (Transformation|GetActorRightVector) 1e+02)))))
    (:then_1
      (Utilities|FlowControl|Delay 0.5)
      (bind _returnvalue_2 (UserInterface|CreateWidget "/Game/WBP_FadeBlack.WBP_FadeBlack_C"))
      (UserInterface|Viewport|AddtoViewport _returnvalue_2 0)
      (Utilities|FlowControl|Delay 1.0)
      (Game|OpenLevel(byObjectReference) "/Game/Maps/MainMap.MainMap"))))

(event Custom|UpSpeed
  (Variables|Default|SetFMultiply (Math|Float|Clamp(Float) (+ (Variables|Default|GetFMultiply) 0.2) 6.0 (Variables|Default|GetMax))))

(event Custom|StartGame
  (Utilities|Time|SetTimerbyEvent (delegate Custom|UpSpeed) 0.2 true)
  (Actor|Tick|SetActorTickEnabled true))

(event EventBeginPlay
  (bind _racineref (Variables|Default|GetRacineRef))
  (bind _spline (Variables|/Game/Blueprints/Interactible/BP_GorowingRoot.BP_GrowingRoot_C|GetSpline _racineref))
  (Transformation|SetActorLocation (Spline|GetLocationatDistanceAlongSpline _spline (Spline|GetSplineLength _spline) "World") false false)
  (Variables|Default|SetCheckpoint (Transformation|GetActorTransform))
  (Utilities|FlowControl|Delay 2e+01)
  (Variables|Default|SetMax 12.0))

(event Collision|EventActorBeginOverlap
  (params (OtherActor :type Actor%20Object%20Reference)))

(event EventTick
  (params (DeltaSeconds :type Float%20%28single-precision%29))
  (bind _returnvalue (Game|GetPlayerCharacter 0))
  (bind _returnvalue_2 (Transformation|GetActorLocation))
  (bind _returnvalue_3 (Transformation|GetActorLocation _returnvalue))
  (bind _returnvalue_4 (Math|Rotator|FindLookatRotation _returnvalue_2 _returnvalue_3))
  (bind (_roll _pitch _yaw) (Math|Rotator|BreakRotator _returnvalue_4))
  (Transformation|SetActorRotation (Math|Rotator|MakeRotator _roll _pitch (+ _yaw -9e+01)))
  (Transformation|SetActorLocation (+ _returnvalue_2 (* (Math|Vector|GetForwardVector _returnvalue_4) (+ (Variables|Default|GetFMultiply) (Variables|Default|GetAdd)))) false false)
  (if (> (Math|Vector|Distance(Vector) _returnvalue_2 _returnvalue_3) 7e+03)
    (Variables|Default|SetAdd (+ (Variables|Default|GetAdd) (* (Utilities|Time|GetWorldDeltaSeconds) 1.6)))
    (else
      (Variables|Default|SetAdd (Math|Float|Clamp(Float) (- (Variables|Default|GetAdd) (* (Utilities|Time|GetWorldDeltaSeconds) 2.5)) 0.0 99999999999999.0)))))

(fn ConstructionScript)