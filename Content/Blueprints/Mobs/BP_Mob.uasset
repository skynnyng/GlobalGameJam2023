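; Enemy mob character, Ghoul or Lich, whose type selects its aggro montage and range.
; It seeds its blackboard and keeps AI logic stopped until the player first comes within horizontal range.
; Jump attacks move it along a timeline-driven Bezier curve with an attack montage, and a timed cooldown broadcasts its reset.
; Any damage stops the AI, ragdolls the mesh and marks it dead; Respawn restores its starting transform and restarts the AI.
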(event Custom|JumpEvent
  (params (Curve :type Struct%20Bezier%20Curve%20Structure))
  (if (not (Audio|Components|Audio|IsPlaying (Variables|Default|GetJumpTimeline)))
    (Variables|Default|SetBezierCurve Curve)
    (Utilities|FlowControl|Sequence
      (:then_0
        (bind _alpha (Timeline|JumpTimeline PlayFromStart)
          (:Update
            (Transformation|SetActorLocation (.ReturnValue (CallFunction|GetLocationBezier (.curvestart (Variables|Default|GetBezierCurve)) (.curvemid (Variables|Default|GetBezierCurve)) (.curveend (Variables|Default|GetBezierCurve)) _alpha 0 0 0 "NewEnumerator3" 0.0 "0, 0, 0" 0 (Utilities|Array|MakeArray ""))) false false))))
      (:then_1
        (Animation|Montage|PlayMontage (Variables|Character|GetMesh) "/Game/Characters/Ghoul/Animations/AM_Attack_Right.AM_Attack_Right")))))

(event Custom|CDJumpReset
  (Variables|Default|SetCDJump false)
  (Default|CallEDResetCDJump))

(event Custom|CDJumpEvent
  (Utilities|Time|SetTimerbyEvent (delegate Custom|CDJumpReset) 5.0)
  (Variables|Default|SetCDJump true))

(event Custom|Respawn
  (bind _mesh (Variables|Character|GetMesh))
  (CallFunction|ResetHitSound)
  (Transformation|SetActorTransform (Variables|Default|GetinitTransform))
  (Class|BrainComponent|RestartLogic (Variables|/Script/AIModule.AIController|GetBrainComponent (AI|GetAIController self)))
  (Physics|SetSimulatePhysics _mesh false)
  (Transformation|SetRelativeTransform _mesh (Math|Transform|MakeTransform "0, 0, 0" "0.000000,-90.000000,0.000000" "1.000000,1.000000,1.000000") false false)
  (Variables|Default|Setded false))

(event Custom|PlayHit
  (Utilities|FlowControl|DoOnce false
    (:Completed
      (Audio|Components|Audio|Play (Variables|Default|GetHIT) 0.32))))

(event Custom|ResetHitSound
  (Utilities|FlowControl|DoOnce false) ; enters at Reset
)

(event EventBeginPlay
  (CallFunction|InitBlackboardValues)
  (Variables|Default|SetinitTransform (Transformation|GetActorTransform))
  (AI|Logic|StopLogic (Variables|/Script/AIModule.AIController|GetBrainComponent (AI|GetAIController self)) ""))

(event EventTick
  (params (DeltaSeconds :type Float%20%28single-precision%29))
  (bind _returnvalue (Game|GetPlayerCharacter 0))
  (bind _self self)
  (bind _returnvalue_2 (Transformation|GetActorLocation _returnvalue))
  (bind _returnvalue_3 (Transformation|GetActorLocation _self))
  (Utilities|IsValid _returnvalue
    (:Is%20Valid
      (Utilities|FlowControl|Sequence
        (:then_0
          (if (< (.z (Transformation|GetVelocity)) 5e+01)
            (Variables|Default|SetjumpStart false)))
        (:then_1
          (if (< (Math|Vector|Distance(Vector) (Math|Vector|MakeVector (.x _returnvalue_2) (.y _returnvalue_2) 0.0) (Math|Vector|MakeVector (.x _returnvalue_3) (.y _returnvalue_3) 0.0)) 4e+03)
            (Utilities|FlowControl|DoOnce false
              (:Completed
                (Class|BrainComponent|RestartLogic (Variables|/Script/AIModule.AIController|GetBrainComponent (AI|GetAIController self)))))))))))

(event Game|Damage|EventAnyDamage
  (params (Damage :type Float%20%28single-precision%29) (DamageType :type Damage%20Type%20Object%20Reference) (InstigatedBy :type Controller%20Object%20Reference) (DamageCauser :type Actor%20Object%20Reference))
  (bind _mesh (Variables|Character|GetMesh))
  (AI|Logic|StopLogic (Variables|/Script/AIModule.AIController|GetBrainComponent (AI|GetAIController self)) "")
  (Collision|SetCollisionResponsetoChannel _mesh "ECC_WorldStatic" "ECR_Block")
  (Collision|SetCollisionResponsetoChannel _mesh "ECC_Pawn" "ECR_Block")
  (Physics|SetSimulatePhysics (Variables|Character|GetMesh) true)
  (Variables|Default|Setded true))

(fn ConstructionScript
  (bind _mobtype (Variables|Default|GetmobType))
  (Variables|Default|SetAggroMontage (Utilities|Select :Index _mobtype :NewEnumerator0 "/Game/Characters/Ghoul/Animations/AM_Ghoul_Aggro.AM_Ghoul_Aggro" :NewEnumerator1 "/Game/Characters/Lich/Animations/AM_LichAggro.AM_LichAggro"))
  (Variables|Default|SetRange (Utilities|Select :Index _mobtype :NewEnumerator0 3.5e+02 :NewEnumerator1 7e+02))
  (Audio|Components|Audio|SetSound (Variables|Default|GetHIT) (Utilities|Select :Index _mobtype :NewEnumerator0 "/Game/Sounds/Mobs/Hits/Sound_player_hit_undead.Sound_player_hit_undead" :NewEnumerator1 "/Game/Sounds/Mobs/Hits/Sound_player_hit_undead.Sound_player_hit_undead")))

(fn InitBlackboardValues
  (bind _returnvalue (AI|GetBlackboard 0))
  (Utilities|IsValid _returnvalue
    (:Is%20Valid
      (AI|Components|Blackboard|SetValueasFloat _returnvalue (Utilities|Name|MakeLiteralName "Range") (Variables|Default|GetRange))
      (AI|Components|Blackboard|SetValueasEnum _returnvalue (Utilities|Name|MakeLiteralName "mobType") (Variables|Default|GetmobType))
      (AI|Components|Blackboard|SetValueasObject _returnvalue (Utilities|Name|MakeLiteralName "player") (Game|GetPlayerCharacter 0)))))