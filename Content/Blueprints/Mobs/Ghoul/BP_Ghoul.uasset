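; Ghoul mob Blueprint that damages the player on contact and randomizes its outfit.
; The construction script binds the modular clothing meshes to the body mesh as leader pose, then randomly toggles visibility of each piece, hair included.
; A capsule overlap with BP_Player applies a fixed point of damage; BeginPlay only calls the parent.
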(event OnComponentBeginOverlap(CapsuleComponent)
  (params (OverlappedComponent :type Primitive%20Component%20Object%20Reference) (OtherActor :type Actor%20Object%20Reference) (OtherComp :type Primitive%20Component%20Object%20Reference) (OtherBodyIndex :type Integer) (bFromSweep :type Boolean) (SweepResult :type Hit%20Result%20Structure%20%28by%20ref%29))
  (bind _asbp_player (Utilities|Casting|CastToBP_Player OtherActor))
  (Game|Damage|ApplyDamage _asbp_player 1.0 0 0))

(event EventBeginPlay
  (|CallParentFunction))

(event Collision|EventActorBeginOverlap
  (params (OtherActor :type Actor%20Object%20Reference)))

(event EventTick
  (params (DeltaSeconds :type Float%20%28single-precision%29)))

(fn ConstructionScript
  (bind _returnvalue (Math|Random|RandomBool))
  (|CallParentFunction)
  (Components|SkinnedMesh|SetLeaderPoseComponent (Variables|Default|GetArmor) (Variables|Character|GetMesh) true false)
  (Variables|Decor|SetRagVisibility _returnvalue)
  (Variables|Decor|SetPantsVisibility _returnvalue)
  (Variables|Decor|SetNeckRopeVisibility _returnvalue)
  (Variables|Decor|SetMaskVisibility _returnvalue)
  (Variables|Decor|SetHairVisibility _returnvalue)
  (Variables|Decor|SetBootsVisibility _returnvalue)
  (Variables|Decor|SetBeltVisibility _returnvalue)
  (Variables|Decor|SetArmorVisibility _returnvalue)
  (Variables|Decor|SetArrowsVisibility _returnvalue)
  (Utilities|FlowControl|Sequence
    (:then_0
      (Rendering|SetVisibility (Variables|Default|GetRag) (Variables|Decor|GetRagVisibility) false))
    (:then_1
      (Rendering|SetVisibility (Variables|Default|GetPants) (Variables|Decor|GetPantsVisibility) false))
    (:then_2
      (Rendering|SetVisibility (Variables|Default|GetNeck_Rope) (Variables|Decor|GetNeckRopeVisibility) false))
    (:then_3
      (Rendering|SetVisibility (Variables|Default|GetMask) (Variables|Decor|GetMaskVisibility) false))
    (:then_4
      (Rendering|SetVisibility (Variables|Default|GetHair) (Variables|Decor|GetHairVisibility) false))
    (:then_5
      (Rendering|SetVisibility (Variables|Default|GetBoots) (Variables|Decor|GetBootsVisibility) false))
    (:then_6
      (Rendering|SetVisibility (Variables|Default|GetBelt) (Variables|Decor|GetBeltVisibility) false))
    (:then_7
      (Rendering|SetVisibility (Variables|Default|GetArrows) (Variables|Decor|GetArrowsVisibility) false))
    (:then_8
      (Rendering|SetVisibility (Variables|Default|GetArmor) (Variables|Decor|GetArmorVisibility) false))))