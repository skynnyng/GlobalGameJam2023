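; Lich mob projectile that grows in, then flies in a straight line through the player's position.
; SummonTimeline scales the Niagara effect and drives its SwirlScale parameter.
; When it finishes, the player's position is sampled once and extrapolated to twice the distance, so the shot overshoots without homing.
; The Movement timeline, sped by PlayRate, lerps the actor there without sweeping; this graph handles no hits, damage or destruction.
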(event EventBeginPlay
  (bind _niagara (Variables|Default|GetNiagara))
  (bind (_direction _x _y _z) (Timeline|SummonTimeline PlayFromStart)
    (:Update
      (Transformation|SetWorldScale3D _niagara (Math|Vector|MakeVector _x _y _z))
      (Class|NiagaraComponent|SetVariableVec2 _niagara "SwirlScale" (Math|Vector2D|MakeVector2D _x _z)))
    (:Finished
      (Variables|Default|SetTarget (Math|Vector|Lerp(Vector) (Transformation|GetActorLocation) (Transformation|GetActorLocation (Game|GetPlayerCharacter 0)) 2.0))
      (Components|Timeline|SetPlayRate (Variables|Default|GetMovement) (Variables|Default|GetplayRate))
      (Variables|Default|Setstart (Transformation|GetActorLocation))
      (bind _alpha (Timeline|Movement PlayFromStart)
        (:Update
          (Transformation|SetActorLocation (Math|Vector|Lerp(Vector) (Variables|Default|Getstart) (Variables|Default|GetTarget) _alpha) false false))))))

(event EventTick
  (params (DeltaSeconds :type Float%20%28single-precision%29)))

(fn ConstructionScript)