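; BP_StartFade is a trigger box that starts a crossfade in the player's ambient music.
; It caches BP_Player on BeginPlay, and any overlap with the box starts a looping timer without checking the actor.
; Each tick of that timer raises the "Crossfade" float parameter on AmbientMusic, prints the value and clears the timer once it reaches Max.
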(event OnComponentBeginOverlap(Box)
  (params (OverlappedComponent :type Primitive%20Component%20Object%20Reference) (OtherActor :type Actor%20Object%20Reference) (OtherComp :type Primitive%20Component%20Object%20Reference) (OtherBodyIndex :type Integer) (bFromSweep :type Boolean) (SweepResult :type Hit%20Result%20Structure%20%28by%20ref%29))
  (bind _returnvalue (Utilities|Time|SetTimerbyEvent (delegate Custom|Fade) 0.1 true))
  (Variables|Default|SetFadeTime _returnvalue))

(event Custom|Fade
  (bind _output_get (Variables|Default|SetCurrent (+ (Variables|Default|GetCurrent) 0.05)))
  (Audio|Parameter|SetFloatParameter (Variables|/Game/Blueprints/Player/BP_Player.BP_Player_C|GetAmbientMusic (Variables|Default|GetAs%20BP%20Player)) "Crossfade" _output_get :!class /Script/Engine.AudioComponent)
  (Development|PrintString (Utilities|String|ToString(Float) _output_get))
  (if (>= _output_get (Variables|Default|GetMax))
    (Utilities|Time|ClearandInvalidateTimerbyHandle (Variables|Default|GetFadeTime))))

(event EventBeginPlay
  (bind _asbp_player (Utilities|Casting|CastToBP_Player (Game|GetPlayerCharacter 0)))
  (Variables|Default|SetAs%20BP%20Player _asbp_player))

(fn ConstructionScript)