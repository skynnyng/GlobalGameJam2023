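; Player controller that owns the root UI layer and handles pausing the game.
; On BeginPlay it adds a CommonUI base widget to the viewport, whose Base container hosts activatable widgets.
; Escape or P toggles pause, deactivating the active widget, then either pushing the pause menu with UI-only input and cursor, or restoring game-only input.
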(event Custom|PauseGame
  (bind _widgetbaseref (Variables|Default|GetWidgetBaseRef))
  (bind _base (Variables|/Game/Blueprints/Widgets/WBP_CommonBase.WBP_CommonBase_C|GetBase _widgetbaseref))
  (Class|CommonActivatableWidget|DeactivateWidget (Class|CommonActivatableWidgetContainerBase|GetActiveWidget (Variables|/Game/Blueprints/Widgets/WBP_CommonBase.WBP_CommonBase_C|GetBase (Variables|Default|GetWidgetBaseRef))))
  (if (not (Game|IsGamePaused))
    (bind _returnvalue (Game|SetGamePaused true))
    (bind _returnvalue_2 (Class|CommonActivatableWidgetContainerBase|AddWidget _base "/Game/Blueprints/Widgets/WBP_PauseMenu.WBP_PauseMenu_C"))
    (Input|SetInputModeUIOnly self _returnvalue_2 "DoNotLock" _returnvalue)
    (Variables|Default|SetbShowMouseCursor true)
    (else
      (Game|SetGamePaused false)
      (Class|CommonActivatableWidget|DeactivateWidget (Class|CommonActivatableWidgetContainerBase|GetActiveWidget _base))
      (Input|SetInputModeGameOnly self false)
      (Variables|Default|SetbShowMouseCursor false))))

(event EventBeginPlay
  (bind _returnvalue (UserInterface|CreateWidget "/Game/Blueprints/Widgets/WBP_CommonBase.WBP_CommonBase_C"))
  (bind _output_get (Variables|Default|SetWidgetBaseRef _returnvalue))
  (UserInterface|Viewport|AddtoViewport _output_get 0))

(event Input|KeyboardEvents|Escape
  (params (Key :type Key%20Structure :default "None"))
  (:Pressed
    (CallFunction|PauseGame)))

(event Input|KeyboardEvents|P
  (params (Key :type Key%20Structure :default "None"))
  (:Pressed
    (CallFunction|PauseGame)))

(fn ConstructionScript)