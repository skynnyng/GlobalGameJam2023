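; An anim notify state that prepares a rotation adjustment for the player toward a configured yaw during an animation.
; On begin, it hands ABP_Player the notify's duration and the yaw delta between ReachingRotation and the rotation from CalculatePlayerRotation.
; The notify only stores these values: its tick is empty, and the per-frame code that would rotate the character is disconnected.
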(fn ReceivedNotifyBegin
  (params (MeshComp :type Skeletal%20Mesh%20Component%20Object%20Reference) (Animation :type Anim%20Sequence%20Base%20Object%20Reference) (TotalDuration :type Float%20%28single-precision%29) (EventReference :type Anim%20Notify%20Event%20Reference%20Structure%20%28by%20ref%29))
  (Utilities|Casting|CastToBP_Player (Components|GetOwner MeshComp)
    (:then
      (bind _asabp_player (Utilities|Casting|CastToABP_Player (Components|SkeletalMesh|GetAnimInstance MeshComp))
        (:then
          (Variables|/Game/Blueprints/Player/ABP_Player.ABP_Player_C|SetRotationTimeAvailable _asabp_player TotalDuration)
          (Variables|/Game/Blueprints/Player/ABP_Player.ABP_Player_C|SetTargetedRotationDelta _asabp_player (.yaw (Math|Rotator|Delta(Rotator) (Math|Rotator|MakeRotator 0.0 0.0 (Variables|Default|GetReachingRotation)) (Math|Rotator|MakeRotator 0.0 0.0 (Default|CalculatePlayerRotation _asabp_player)))))
          (return true))
        (:CastFailed
          _)))
    (:CastFailed
      _))
  (return false))

(fn ReceivedNotifyTick
  (params (MeshComp :type Skeletal%20Mesh%20Component%20Object%20Reference) (Animation :type Anim%20Sequence%20Base%20Object%20Reference) (FrameDeltaTime :type Float%20%28single-precision%29) (EventReference :type Anim%20Notify%20Event%20Reference%20Structure%20%28by%20ref%29)))