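; BP_Skills implements the player's skills as callable events acting on a cached BP_Player: wave attack, homing strike, big slash and double jump.
; ThirdAttack, gated by DoOnce, moves a Niagara wave along world X on a timeline, box-tracing for BP_Mob targets.
; Homing lerps the player to a mob at distance-scaled speed, damages it, then launches away with collision briefly disabled.
; BigSlash sphere-traces for damage; DoubleJump raises jump count.
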(event Custom|ThirdAttack
  (bind _playerref (Variables|Default|GetPlayerRef))
  (Utilities|FlowControl|DoOnce false
    (:Completed
      (Animation|Montage|PlayMontage (Variables|/Script/Engine.Character|GetMesh _playerref) "/Game/Characters/Mannequins/Mixamo/Animations/Attack_Up_01_Seq_Montage.Attack_Up_01_Seq_Montage"
        (:OnNotifyBegin
          (bind _returnvalue (Niagara|SpawnSystematLocation "/Game/FX/NiagaraSystem/NS_WaveAttackTEMP.NS_WaveAttackTEMP" (Transformation|GetActorLocation _playerref)))
          (bind _output_get (Variables|Default|SetWave _returnvalue))
          (Variables|Default|SetWaveLoc (Transformation|GetWorldLocation _output_get))
          (bind _alpha (Timeline|WaveT PlayFromStart)
            (:Update
              (Variables|Default|SetLocation (Math|Vector|Lerp(Vector) (Variables|Default|GetWaveLoc) (Math|Vector|MakeVector (+ (.x (Variables|Default|GetWaveLoc)) 1e+03) (.y (Variables|Default|GetWaveLoc)) (.z (Variables|Default|GetWaveLoc))) _alpha))
              (Transformation|SetWorldLocation (Variables|Default|GetWave) (Variables|Default|GetLocation) false false)
              (bind (_outhit _returnvalue_2) (Class|KismetSystemLibrary|BoxTraceSingleforObjects (Variables|Default|GetLocation) (Variables|Default|GetLocation) "100.000000,100.000000,20.000000" "0, 0, 0" (Utilities|Array|MakeArray "ObjectTypeQuery3") false 0 "ForOneFrame" true))
              (if _returnvalue_2
                (bind _asbp_mob (Utilities|Casting|CastToBP_Mob (.HitActor (Collision|BreakHitResult _outhit))))
                (Game|Damage|ApplyDamage _asbp_mob 0.0 0 0)))
            (:Finished
              (Components|DestroyComponent (Variables|Default|GetWave))
              (CallFunction|ResetAttack))))))))

(event Custom|Homing
  (params (MobRef :type BP%20Mob%20Object%20Reference))
  (bind _playerref (Variables|Default|GetPlayerRef))
  (bind _playerref_2 (Variables|Default|GetPlayerRef))
  (bind _capsulecomponent (Variables|/Script/Engine.Character|GetCapsuleComponent _playerref))
  (bind _mesh (Variables|/Script/Engine.Character|GetMesh _playerref_2))
  (Variables|Default|SetMob%20Ref MobRef)
  (Animation|Montage|PlayMontage _mesh "/Game/Characters/Mannequins/Mixamo/Animations/Attack_Air_To_Floor_Start_03_Seq_Montage.Attack_Air_To_Floor_Start_03_Seq_Montage"
    (:then
      (Animation|Montage|PlayMontage _mesh "/Game/Characters/Mannequins/Mixamo/Animations/Attack_Air_To_Floor_Loop_03_Seq_Montage.Attack_Air_To_Floor_Loop_03_Seq_Montage"
        (:then
          (Variables|Default|SetPlayerLoc (Transformation|GetActorLocation (Variables|Default|GetPlayerRef)))
          (Components|Timeline|SetPlayRate (Variables|Default|GetHomingT) (Math|Float|MapRangeClamped (Transformation|GetDistanceTo (Variables|Default|GetPlayerRef) (Variables|Default|GetMob%20Ref)) 1e+02 2e+03 1e+01 1.0))
          (bind _alpha (Timeline|HomingT PlayFromStart)
            (:Update
              (Transformation|SetActorLocation (Variables|Default|GetPlayerRef) (Math|Vector|Lerp(Vector) (Variables|Default|GetPlayerLoc) (Math|Vector|MakeVector (.x (Transformation|GetActorLocation (Variables|Default|GetMob%20Ref))) (.y (Transformation|GetActorLocation (Variables|Default|GetMob%20Ref))) (.z (Transformation|GetActorLocation (Variables|Default|GetMob%20Ref)))) _alpha) false false))
            (:Finished
              (Game|Damage|ApplyDamage (Variables|Default|GetMob%20Ref) 0.0 0 0)
              (Animation|Montage|PlayMontage (Variables|/Script/Engine.Character|GetMesh _playerref) "/Game/Characters/Mannequins/Mixamo/Animations/Attack_Air_To_Floor_End_03_Seq_Montage.Attack_Air_To_Floor_End_03_Seq_Montage"
                (:then
                  (Collision|SetCollisionEnabled _capsulecomponent "NoCollision")
                  (Character|LaunchCharacter _playerref (Math|Vector|MakeVector 1e+03 0.0 1e+03) true true)
                  (Utilities|FlowControl|Delay 0.2)
                  (Collision|SetCollisionEnabled _capsulecomponent "QueryAndPhysics"))))))))))

(event Custom|BigSlash
  (bind _playerref (Variables|Default|GetPlayerRef))
  (bind _returnvalue (Transformation|GetActorLocation _playerref))
  (Animation|Montage|PlayMontage (Variables|/Script/Engine.Character|GetMesh (Variables|Default|GetPlayerRef)) "/Game/Characters/Mannequins/Mixamo/Animations/Combo_Attack_03_01_Seq_Montage.Combo_Attack_03_01_Seq_Montage"
    (:then
      (bind (_outhit _returnvalue_2) (Collision|SphereTraceForObjects _returnvalue _returnvalue 2e+02 (Utilities|Array|MakeArray "ObjectTypeQuery3") false 0 "ForDuration"))
      (if _returnvalue_2
        (bind _asbp_mob (Utilities|Casting|CastToBP_Mob (.HitActor (Collision|BreakHitResult _outhit))))
        (Game|Damage|ApplyDamage _asbp_mob 0.0 0 0)
        (Development|PrintString "Hello")))))

(event Custom|ResetAttack
  (bind _playerref (Variables|Default|GetPlayerRef))
  (Utilities|FlowControl|DoOnce false) ; enters at Reset
)

(event Custom|DoubleJump
  (Variables|/Script/Engine.Character|SetJumpMaxCount (Variables|Default|GetPlayerRef) 2))

(event EventBeginPlay
  (bind _asbp_player (Utilities|Casting|CastToBP_Player (Game|GetPlayerCharacter 0)))
  (Variables|Default|SetPlayerRef _asbp_player))

(fn ConstructionScript)