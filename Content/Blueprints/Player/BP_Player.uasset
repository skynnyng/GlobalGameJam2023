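; Player character with Enhanced Input movement, jump, montage-driven slide, grapple and sword combat.
; Spawns BP_Skills and CA_Grapple helper actors; attacks choose between combo montage, slide slash, unlockable finisher and airborne homing onto living mobs found by sphere trace.
; HitEvent box-traces at the sword socket to damage mobs, while taking damage grants temporary invulnerability with timeline-driven material and walk-speed effects.
; Respawn restores the checkpoint transform, respawns mobs and destroys projectiles.
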(event Custom|Slide
  (Pawn|Input|AddMovementInput (Variables|Default|GetVelocity) 1e+02 false))

(event Custom|ResetDamage
  (Variables|Actor|SetbCanBeDamaged true))

(event Custom|Start
  (bind _returnvalue (Audio|SpawnSound2D "/Game/Sounds/Musics/SC_Music.SC_Music" 1.0 1.0 0.0 0))
  (Variables|Default|SetAmbientMusic _returnvalue))

(event Custom|ResetMontage
  (bind _mesh (Variables|Character|GetMesh))
  (bind _returnvalue (Components|SkeletalMesh|GetAnimInstance _mesh))
  (Animation|Montage|MontageStop _returnvalue 0.25 (Animation|Montage|GetCurrentActiveMontage _returnvalue)))

(event Input|EnhancedActionEvents|EnhancedInputActionIA_Move
  (params (ActionValue :type Vector%202D%20Structure) (ElapsedSeconds :type Float%20%28double-precision%29) (TriggeredSeconds :type Float%20%28double-precision%29) (InputAction :type Input%20Action%20Object%20Reference :default "/Game/Blueprints/Player/Inputs/IA_Move.IA_Move"))
  (bind _returnvalue (Pawn|GetControlRotation :!class /Script/Engine.Pawn))
  (:Triggered
    (bind _output_get (Variables|Default|SetforwardInputDirection (Math|Vector|GetForwardVector (Math|Rotator|MakeRotator 0.0 0.0 (.yaw _returnvalue)))))
    (Pawn|Input|AddMovementInput _output_get (* (.x ActionValue) -1.0) false)
    (Pawn|Input|AddMovementInput (Math|Vector|GetRightVector (Math|Rotator|MakeRotator (.roll _returnvalue) 0.0 (.yaw _returnvalue))) (.y ActionValue) false)))

(event Input|EnhancedActionEvents|EnhancedInputActionIA_Look
  (params (ActionValue :type Vector%202D%20Structure) (ElapsedSeconds :type Float%20%28double-precision%29) (TriggeredSeconds :type Float%20%28double-precision%29) (InputAction :type Input%20Action%20Object%20Reference :default "/Game/Blueprints/Player/Inputs/IA_Look.IA_Look"))
  (:Triggered
    (Pawn|Input|AddControllerYawInput (.x ActionValue))
    (Pawn|Input|AddControllerPitchInput (* (.y ActionValue) -1.0))))

(event Input|EnhancedActionEvents|EnhancedInputActionIA_Grab
  (params (ActionValue :type Boolean) (ElapsedSeconds :type Float%20%28double-precision%29) (TriggeredSeconds :type Float%20%28double-precision%29) (InputAction :type Input%20Action%20Object%20Reference :default "/Game/Blueprints/Player/Inputs/IA_Grab.IA_Grab"))
  (:Started
    (if (Variables|Actor|GetbCanBeDamaged)
      (Default|StartGrab (Variables|Default|GetGrapple)))))

(event Input|EnhancedActionEvents|EnhancedInputActionIA_Slide
  (params (ActionValue :type Boolean) (ElapsedSeconds :type Float%20%28double-precision%29) (TriggeredSeconds :type Float%20%28double-precision%29) (InputAction :type Input%20Action%20Object%20Reference :default "/Game/Blueprints/Player/Inputs/IA_Slide.IA_Slide"))
  (bind _returnvalue (Input|EnhancedActionValues|GetIA_Move))
  (bind _charactermovement (Variables|Character|GetCharacterMovement))
  (bind _capsulecomponent (Variables|Collision|GetCapsuleComponent))
  (bind _capsulecomponent_2 (Variables|Collision|GetCapsuleComponent))
  (bind _charactermovement_2 (Variables|Character|GetCharacterMovement))
  (:Started
    (if (Math|Boolean|ANDBoolean (or (!= (.x _returnvalue) 0.0) (!= (.y _returnvalue) 0.0)) (Variables|Default|GetCanSlide) (not (Variables|/Game/Blueprints/Interactible/CA_Grapple.CA_Grapple_C|GetinGrapple (Variables|Default|GetGrapple))) (Variables|Actor|GetbCanBeDamaged))
      (Components|Capsule|SetCapsuleHalfHeight _capsulecomponent_2 (/ (Variables|/Script/Engine.CapsuleComponent|GetCapsuleHalfHeight _capsulecomponent_2) 2.0) true)
      (Transformation|SetRelativeLocation (Variables|Character|GetMesh) "0.000000,0.000000,-45.000000" false false)
      (Variables|Default|SetdoingThings true)
      (Variables|Default|SetSliding true)
      (Animation|Montage|PlayMontage (Variables|Character|GetMesh) "/Game/Characters/Mannequins/Animations/Player/Slide_Montage.Slide_Montage"
        (:then
          (Variables|Default|SetVelocity (Transformation|GetActorForwardVector))
          (bind _returnvalue_2 (Utilities|Time|SetTimerbyEvent (delegate Custom|Slide) 0.01 true))
          (Variables|Default|SetTimer _returnvalue_2)
          (Variables|Default|SetCanSlide false)
          (Variables|/Script/Engine.CharacterMovementComponent|SetbOrientRotationToMovement _charactermovement false)
          (Variables|/Script/Engine.CharacterMovementComponent|SetbUseControllerDesiredRotation _charactermovement false))
        (:OnCompleted
          (Utilities|Time|ClearandInvalidateTimerbyHandle (Variables|Default|GetTimer) :!label _label)
          (Variables|Default|SetCanSlide true)
          (Variables|/Script/Engine.CharacterMovementComponent|SetbOrientRotationToMovement _charactermovement_2 true)
          (Variables|/Script/Engine.CharacterMovementComponent|SetbUseControllerDesiredRotation _charactermovement_2 true)
          (Variables|Default|SetSliding false)
          (Components|Capsule|SetCapsuleHalfHeight _capsulecomponent (* (Variables|/Script/Engine.CapsuleComponent|GetCapsuleHalfHeight _capsulecomponent) 2.0) false)
          (Transformation|AddActorWorldOffset "0.000000,0.000000,50.000000")
          (Transformation|SetRelativeLocation (Variables|Character|GetMesh) "0.000000,0.000000,-90.000000" false false)
          (Utilities|FlowControl|Delay 0.7)
          (Variables|Default|SetdoingThings false))
        (:OnInterrupted
          (goto _label))))))

(event Input|EnhancedActionEvents|EnhancedInputActionIA_Attack
  (params (ActionValue :type Boolean) (ElapsedSeconds :type Float%20%28double-precision%29) (TriggeredSeconds :type Float%20%28double-precision%29) (InputAction :type Input%20Action%20Object%20Reference :default "/Game/Blueprints/Player/Inputs/IA_Attack.IA_Attack"))
  (bind _mesh (Variables|Character|GetMesh))
  (bind _mesh_2 (Variables|Character|GetMesh))
  (bind _returnvalue (Components|SkeletalMesh|GetAnimInstance _mesh))
  (bind _returnvalue_2 (Components|SkeletalMesh|GetAnimInstance _mesh_2))
  (bind _returnvalue_3 (Animation|Montage|MontageGetPosition _returnvalue 0))
  (:Started
    (if (and (not (Variables|/Game/Blueprints/Interactible/CA_Grapple.CA_Grapple_C|GetinGrapple (Variables|Default|GetGrapple))) (Variables|Actor|GetbCanBeDamaged))
      (Animation|Montage|MontageSetPlayRate _returnvalue 0 1.0)
      (Utilities|Time|ClearandInvalidateTimerbyHandle (Variables|Default|GetTimerMontage))
      (if (and (Variables|Default|GetHomingUnlocked) (AI|Components|NavMovement|IsFalling (Variables|Character|GetCharacterMovement)))
        (bind (_returnvalue_4 _returnvalue2) (CallFunction|FindEnemyHomming))
        (Development|PrintString "1")
        (Utilities|IsValid _returnvalue_4
          (:Is%20Valid
            (Development|PrintString "2")
            (Transformation|SetActorRotation (Math|Rotator|MakeRotator 0.0 0.0 (.yaw (Math|Rotator|FindLookatRotation _returnvalue2 (Transformation|GetActorLocation _returnvalue_4)))))
            (Development|PrintString "3")
            (bind _asbp_mob (Utilities|Casting|CastToBP_Mob _returnvalue_4))
            (Development|PrintString "4")
            (Default|Homing (Variables|Default|GetSkillsRef) _asbp_mob))
          (:Is%20Not%20Valid
            (if (Variables|Default|GetSliding) :!label _label
              (Default|BigSlash (Variables|Default|GetSkillsRef))
              (elif (not (Class|AnimInstance|IsAnyMontagePlaying _returnvalue))
                (bind _notifyname (Animation|Montage|PlayMontage (Variables|Character|GetMesh) "/Game/TESTCOMBOA_Montage.TESTCOMBOA_Montage" 3.0 :!label _label_2)
                  (:OnNotifyBegin
                    (switch name _notifyname
                      (:A
                        _)
                      (:B
                        _))
                    (Animation|Montage|MontageSetPlayRate _returnvalue_2 (Animation|Montage|GetCurrentActiveMontage _returnvalue_2) 0.08)
                    (bind _returnvalue_5 (Utilities|Time|SetTimerbyEvent (delegate Custom|ResetMontage) 1.0))
                    (Variables|Default|SetTimerMontage _returnvalue_5)))
                (elif (> _returnvalue_3 1.38)
                  (goto _label_2)
                  (elif (Math|Boolean|ANDBoolean (> _returnvalue_3 0.65) (Variables|Default|GetFinisherUnlocked) (== (Animation|Montage|GetCurrentActiveMontage _returnvalue) "/Game/TESTCOMBOA_Montage.TESTCOMBOA_Montage"))
                    (Default|ThirdAttack (Variables|Default|GetSkillsRef))))))))
        (else
          (goto _label))))))

(event Input|EnhancedActionEvents|EnhancedInputActionIA_Jump
  (params (ActionValue :type Boolean) (ElapsedSeconds :type Float%20%28double-precision%29) (TriggeredSeconds :type Float%20%28double-precision%29) (InputAction :type Input%20Action%20Object%20Reference :default "/Game/Blueprints/Player/Inputs/IA_Jump.IA_Jump"))
  (bind _mesh (Variables|Character|GetMesh))
  (bind _charactermovement (Variables|Character|GetCharacterMovement))
  (bind _returnvalue (Components|SkeletalMesh|GetAnimInstance _mesh))
  (:Started
    (bind _grapple (Variables|Default|GetGrapple)
      (:then
        (if (not (Variables|/Game/Blueprints/Interactible/CA_Grapple.CA_Grapple_C|GetinGrapple _grapple))
          (Character|Jump)
          (if (Class|AnimInstance|IsAnyMontagePlaying _returnvalue)
            (Animation|StopAnimMontage (Animation|Montage|GetCurrentActiveMontage _returnvalue)))
          (Variables|Default|SetCanSlide false)
          (Variables|/Script/Engine.CharacterMovementComponent|SetbOrientRotationToMovement _charactermovement false)
          (Variables|/Script/Engine.CharacterMovementComponent|SetbUseControllerDesiredRotation _charactermovement false)
          (Audio|PlaySound2D 0 1.0 1.0 0.0 0 0)))
      (:else)))
  (:Completed
    (Character|StopJumping)))

(event EventBeginPlay
  (Input|AddMappingContext (PlayerController|LocalPlayerSubsystems|GetEnhancedInputLocalPlayerSubsystem (Game|GetPlayerController 0)) "/Game/Blueprints/Player/Inputs/IMC_Player.IMC_Player" 0 "(bIgnoreAllPressedKeysUntilRelease=True,bForceImmediately=False)")
  (bind _returnvalue (Game|SpawnActorfromClass "/Game/Blueprints/Player/BP_Skills.BP_Skills_C" (Transformation|GetActorTransform) "Undefined" 0 0))
  (bind _output_get (Variables|Default|SetSkillsRef _returnvalue))
  (Transformation|AttachActorToActor _output_get self "None" "KeepRelative" "KeepRelative" "KeepRelative" true)
  (bind _returnvalue_2 (Game|SpawnActorfromClass "/Game/Blueprints/Interactible/CA_Grapple.CA_Grapple_C" (Math|Transform|MakeTransform "0, 0, 0" "0, 0, 0" "1.000000,1.000000,1.000000") "Undefined" 0 0))
  (Variables|Default|SetGrapple _returnvalue_2)
  (Variables|Default|SetCheckpoint (Transformation|GetActorTransform))
  (bind _returnvalue_3 (Rendering|Material|CreateDynamicMaterialInstance (Variables|Default|GetSword) 0 "/Game/Characters/Mannequins/Materials/MAT_Player.MAT_Player" "None" :!class /Script/Engine.PrimitiveComponent))
  (Utilities|Array|AddUnique (Variables|Default|GetDynamicMats) _returnvalue_3)
  (for (_ _array_index) (Rendering|Material|GetMaterials (Variables|Character|GetMesh))
    (bind _returnvalue_4 (Rendering|Material|CreateDynamicMaterialInstance (Variables|Character|GetMesh) _array_index "/Game/Characters/Mannequins/Materials/MAT_Player.MAT_Player" "None" :!class /Script/Engine.PrimitiveComponent))
    (Utilities|Array|AddUnique (Variables|Default|GetDynamicMats) _returnvalue_4))
  (bind _outactors (Actor|GetAllActorsOfClass "/Game/Blueprints/Mobs/BP_Mob.BP_Mob_C"))
  (Variables|Default|Setmobs _outactors)
  (Transformation|SetActorLocation "1485.000000,2465.000000,2200.000000" false false)
  (Variables|/Script/Engine.CharacterMovementComponent|SetGravityScale (Variables|Character|GetCharacterMovement) 1.0))

(event EventOnLanded
  (params (Hit :type Hit%20Result%20Structure%20%28by%20ref%29))
  (bind _charactermovement (Variables|Character|GetCharacterMovement))
  (Variables|Default|SetCanSlide true)
  (Variables|/Script/Engine.CharacterMovementComponent|SetbOrientRotationToMovement _charactermovement true)
  (Variables|/Script/Engine.CharacterMovementComponent|SetbUseControllerDesiredRotation _charactermovement true)
  (Character|StopJumping))

(event Game|Damage|EventAnyDamage
  (params (Damage :type Float%20%28single-precision%29) (DamageType :type Damage%20Type%20Object%20Reference) (InstigatedBy :type Controller%20Object%20Reference) (DamageCauser :type Actor%20Object%20Reference))
  (if (Variables|Actor|GetbCanBeDamaged)
    (Variables|Actor|SetbCanBeDamaged false)
    (Components|Activation|Activate (Variables|Default|GetFX_Hit) false)
    (Animation|Montage|PlayMontage (Variables|Character|GetMesh) "/Game/Characters/Mannequins/Animations/Player/AM_Soccer_Trip.AM_Soccer_Trip" 1.5
      (:then
        (for _array_element (Variables|Default|GetDynamicMats)
          (Rendering|Material|SetScalarParameterValue _array_element "Speed" 0.8 :!class /Script/Engine.MaterialInstanceDynamic))
        (bind (_direction _alpha _al) (Timeline|Timeline PlayFromStart)
          (:Update
            (for _array_element_2 (Variables|Default|GetDynamicMats)
              (Rendering|Material|SetScalarParameterValue _array_element_2 "Opacity" (Math|Float|Lerp 0.0 3.0 _al) :!class /Script/Engine.MaterialInstanceDynamic)
              (Rendering|Material|SetScalarParameterValue _array_element_2 "DispAmount" (Math|Float|Lerp 0.0 1e+01 _alpha) :!class /Script/Engine.MaterialInstanceDynamic))
            (Variables|/Script/Engine.CharacterMovementComponent|SetMaxWalkSpeed (Variables|Character|GetCharacterMovement) (Math|Float|Lerp 2.4e+03 6e+02 _alpha)))
          (:Finished
            (Utilities|FlowControl|Delay 0.6)
            (Rendering|Material|SetScalarParameterValue _array_element "Speed" 0.1 :!class /Script/Engine.MaterialInstanceDynamic)
            (bind _newtrack_0 (Timeline|Timeline_0 PlayFromStart)
              (:Update
                (for _array_element_3 (Variables|Default|GetDynamicMats)
                  (Rendering|Material|SetScalarParameterValue _array_element_3 "Opacity" (Math|Float|Lerp 0.0 1.0 _newtrack_0) :!class /Script/Engine.MaterialInstanceDynamic)
                  (Rendering|Material|SetScalarParameterValue _array_element_3 "DispAmount" (Math|Float|Lerp 0.0 1e+01 _newtrack_0) :!class /Script/Engine.MaterialInstanceDynamic))
                (Variables|/Script/Engine.CharacterMovementComponent|SetMaxWalkSpeed (Variables|Character|GetCharacterMovement) (Math|Float|Lerp 2.4e+03 6e+02 _newtrack_0)))
              (:Finished
                (CallFunction|ResetDamage)))))))))

(fn ConstructionScript)

(fn InterruptedAnim
  (if (Math|Boolean|ORBoolean (Variables|Default|GetbPressedJump) (Variables|Default|GetSliding) (Variables|/Game/Blueprints/Interactible/CA_Grapple.CA_Grapple_C|GetinGrapple (Variables|Default|GetGrapple)) (not (Variables|Actor|GetbCanBeDamaged)))
    (Variables|Default|SetCanAttack true)
    (Variables|Default|SetdoingThings false)
    (else
      (Development|PrintString "echec"))))

(fn HitEvent
  (bind _mesh (Variables|Character|GetMesh))
  (bind _returnvalue (Transformation|GetSocketLocation _mesh "SwordSocket"))
  (bind _outhit (Class|KismetSystemLibrary|BoxTraceSingleforObjects _returnvalue _returnvalue "50.000000,50.000000,200.000000" (Transformation|GetSocketRotation _mesh "SwordSocket") (Utilities|Array|MakeArray "ObjectTypeQuery3") false 0 "None" true))
  (bind _asbp_mob (Utilities|Casting|CastToBP_Mob (.HitActor (Collision|BreakHitResult _outhit))))
  (Default|PlayHit _asbp_mob)
  (Game|Damage|ApplyDamage _asbp_mob 1.0 0 0))

(fn Respawn
  (Transformation|SetActorTransform (Variables|Default|GetCheckpoint))
  (for _array_element (Variables|Default|Getmobs)
    (Utilities|IsValid _array_element
      (:Is%20Valid
        (Default|Respawn _array_element))))
  (bind _outactors (Actor|GetAllActorsOfClass "/Game/Blueprints/Mobs/Lich/BP_Projectile.BP_Projectile_C"))
  (for _array_element_2 _outactors
    (Actor|DestroyActor _array_element_2)))

(fn FindEnemyHomming
  (bind _returnvalue (Transformation|GetActorLocation))
  (bind (_outhits _returnvalue_2) (Collision|MultiSphereTraceForObjects _returnvalue (+ _returnvalue "0.000000,0.000000,1.000000") 2e+03 (Utilities|Array|MakeArray "ObjectTypeQuery3") false 0 "None"))
  (if _returnvalue_2
    (for _array_element _outhits
      (bind _asbp_mob (Utilities|Casting|CastToBP_Mob (.HitActor (Collision|BreakHitResult _array_element))))
      (if (not (Variables|/Game/Blueprints/Mobs/BP_Mob.BP_Mob_C|Getded _asbp_mob))
        (return _asbp_mob (Transformation|GetActorLocation))))))